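; Ball actor that travels in a straight line and bounces off the surfaces it hits.
; BeginPlay sets Speed from BaseSpeed, and each Tick moves the actor along Direction with a swept world offset.
; The sweep's hit normal feeds a reflection of Direction every frame, as the branch before it is always true.
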(event EventBeginPlay
  (Variables|Default|Setspeed (Variables|Default|GetBase%20Speed)))

(event Collision|EventActorBeginOverlap
  (params (OtherActor :type Actor%20Object%20Reference)))

(event EventTick
  (params (DeltaSeconds :type Float%20%28single-precision%29))
  (bind _sweephitresult (Transformation|AddActorWorldOffset (* (* (Variables|Default|Getdirection) (Variables|Default|Getspeed)) DeltaSeconds) true))
  (if true
    (Variables|Default|Setdirection (Math|Vector|GetReflectionVector (Variables|Default|Getdirection) (.Normal (Collision|BreakHitResult _sweephitresult))))))

(fn ConstructionScript)