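; Child Blueprint of a parent actor, apparently a destruction object, that rescales itself whenever another actor overlaps it.
; BeginPlay runs the parent logic, then copies BaseScale into Scale.
; On overlap it multiplies the current actor scale uniformly by Multiply into BaseScale, runs the parent overlap handler, then applies BaseScale, so repeated overlaps compound.
; The Tick override is disabled and construction only calls the parent.
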(event EventBeginPlay
  (|CallParentFunction)
  (Variables|Default|SetScale (Variables|Default|GetBase%20Scale)))

(event Collision|EventActorBeginOverlap
  (params (OtherActor :type Actor%20Object%20Reference))
  (bind _multiply (Variables|Default|GetMultiply))
  (bind _output_get (Variables|Default|SetBase%20Scale (Transformation|GetActorScale3D)))
  (bind _output_get_2 (Variables|Default|SetBase%20Scale (* _output_get (Math|Vector|MakeVector _multiply _multiply _multiply))))
  (|CallParentFunction OtherActor)
  (Transformation|SetActorScale3D _output_get_2))

(event EventTick
  (params (DeltaSeconds :type Float%20%28single-precision%29))
  (|CallParentFunction DeltaSeconds) ; This node is disabled and will not be called.\nDrag off pins to build functionality.
)

(fn ConstructionScript
  (|CallParentFunction))